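; BP_PlayerPawn is a player pawn that rolls a sphere and restarts the level when it takes damage.
; Forward/back and left/right axis inputs apply torque to the Sphere around world Y and X, scaled by Multiply and applied as an acceleration change, so mass is ignored.
; Any damage fades the camera out, waits for the fade, then reopens the current level by name.
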(event Game|Damage|EventAnyDamage
  (params (Damage :type Float%20%28single-precision%29) (DamageType :type Damage%20Type%20Object%20Reference) (InstigatedBy :type Controller%20Object%20Reference) (DamageCauser :type Actor%20Object%20Reference))
  (bind _returnvalue (Math|Float|MakeLiteralFloat 1.0))
  (CameraFades|StartCameraFade :self (Game|GetPlayerCameraManager 0) :ToAlpha 1.0 :Duration _returnvalue)
  (Utilities|FlowControl|Delay _returnvalue)
  (bind _returnvalue_2 (Game|GetCurrentLevelName true))
  (Game|OpenLevel(byName) (Utilities|String|StringToName _returnvalue_2)))

(event Input|AxisEvents|InputAxisMovingForwardBack
  (params (AxisValue :type Float%20%28single-precision%29))
  (Class|PrimitiveComponent|AddTorqueinRadians (Variables|Default|GetSphere) (Math|Vector|MakeVector 0.0 (* AxisValue (Variables|Default|GetMultiply)) 0.0) "None" true))

(event Input|AxisEvents|InputAxisMovingLeftRight
  (params (AxisValue :type Float%20%28single-precision%29))
  (Class|PrimitiveComponent|AddTorqueinRadians (Variables|Default|GetSphere) (Math|Vector|MakeVector (* AxisValue (Variables|Default|GetMultiply)) 0.0 0.0) "None" true))

(fn ConstructionScript)