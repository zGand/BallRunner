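; Enemy cannon Blueprint that fires projectiles automatically on a repeating cycle from BeginPlay.
; Each cycle waits FireRate, then spawns a Projectiles actor at the Arrow component's transform, scaled by ProjectileScale.
; A CannonShoot timeline then drives the Cannon component's relative Y location for barrel recoil, and its Finished output loops back to the delay.
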(event EventBeginPlay
  (Utilities|FlowControl|Delay (Variables|CanonProperties|GetFireRate) :!label _label)
  (CallFunction|SpawnProjectile)
  (bind _cannonrecoil (Timeline|CannonShoot PlayFromStart)
    (:Update
      (CallFunction|CanonAnimation _cannonrecoil))
    (:Finished
      (goto _label))))

(fn ConstructionScript)

(fn SpawnProjectile
  (bind _arrow (Variables|Default|GetArrow))
  (Game|SpawnActorfromClass "/Game/Blueprints/Enemy/Projectiles.Projectiles_C" (Math|Transform|MakeTransform (Transformation|GetWorldLocation _arrow) (Transformation|GetWorldRotation _arrow) (Variables|CanonProperties|GetProjectileScale)) "Undefined" 0 0))

(fn CanonAnimation
  (params (CannonBarrelYLocation :type Float%20%28single-precision%29))
  (Transformation|SetRelativeLocation (Variables|Default|GetCannon) (Math|Vector|MakeVector 0.0 CannonBarrelYLocation 0.0) false false))