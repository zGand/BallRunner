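; BP_Crystal is a collectable crystal that plays a pickup animation when the player pawn overlaps its sphere, then destroys itself.
; On overlap it snapshots its location, scale and point light intensity, plus the player's location.
; A timeline's separate tracks drive lerps that move it to that captured position, without following the player, while shrinking it to zero and fading out the light.
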(event OnComponentBeginOverlap(Sphere)
  (params (OverlappedComponent :type Primitive%20Component%20Object%20Reference) (OtherActor :type Actor%20Object%20Reference) (OtherComp :type Primitive%20Component%20Object%20Reference) (OtherBodyIndex :type Integer) (bFromSweep :type Boolean) (SweepResult :type Hit%20Result%20Structure%20%28by%20ref%29))
  (Utilities|IsPlayer OtherActor
    (:IsPlayer
      (CallFunction|SetVariables)
      (bind (_direction _crystallocation _crystal_scale _lightintensity) (Timeline|CrystalTimeione Play)
        (:Update
          (CallFunction|ChangeLocation _crystallocation)
          (CallFunction|ChangeScale _crystal_scale)
          (CallFunction|ChangeLight _lightintensity))
        (:Finished
          (Actor|DestroyActor))))))

(fn ConstructionScript)

(fn ChangeLocation
  (params (Alpha :type Float%20%28single-precision%29))
  (Transformation|SetActorLocation (Math|Vector|Lerp(Vector) (Variables|Default|GetCrystalLocation) (Variables|Default|GetBallLocation) Alpha) false false))

(fn ChangeScale
  (params (Alpha :type Float%20%28single-precision%29))
  (Transformation|SetActorScale3D (Math|Vector|Lerp(Vector) (Variables|Default|GetCrystalScale) "0, 0, 0" Alpha)))

(fn ChangeLight
  (params (Alpha :type Float%20%28single-precision%29))
  (Rendering|Components|Light|SetIntensity (Variables|Default|GetPointLight) (Math|Float|Lerp (Variables|Default|GetCrystalLight) 0.0 Alpha)))

(fn SetVariables
  (Variables|Default|SetCrystalLocation (Transformation|GetActorLocation))
  (Variables|Default|SetCrystalLight (Variables|/Script/Engine.LightComponentBase|GetIntensity (Variables|Default|GetPointLight)))
  (Variables|Default|SetBallLocation (Transformation|GetActorLocation (Game|Player|GetPlayerPawn 0)))
  (Variables|Default|SetCrystalScale (Transformation|GetActorScale3D)))