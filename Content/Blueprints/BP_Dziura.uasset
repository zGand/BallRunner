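; BP_Dziura (Polish for "hole") is a trigger that restarts the current level, likely after a fall.
; BeginPlay fades the camera in from black.
; When any actor ends overlap with the Box, the Fade&Restart graph fades the camera out, waits for the fade to finish, then reopens the current level by name.
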(event OnComponentEndOverlap(Box)
  (params (OverlappedComponent :type Primitive%20Component%20Object%20Reference) (OtherActor :type Actor%20Object%20Reference) (OtherComp :type Primitive%20Component%20Object%20Reference) (OtherBodyIndex :type Integer))
  (bind _returnvalue (Utilities|Fade&Restart (Game|GetPlayerCameraManager 0))))

(event EventBeginPlay
  (CameraFades|StartCameraFade :self (Game|GetPlayerCameraManager 0) :FromAlpha 1.0 :ToAlpha 0.0 :Duration (stale OnComponentEndOverlap(Box) _returnvalue)))

(fn ConstructionScript)